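; BP_Dialogue_component steps through data-table-driven dialogue, advancing one line each time its Interact event fires.
; The first interaction creates a WB_Dialogue widget with the speaker name and current line, and later ones update that widget.
; Each row supplies the next row name, data table and end flag, so conversations chain across tables.
; Once the end flag is set, the next interaction removes the widget and clears that flag.
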(event EventBeginPlay)

(event EventTick
  (params (DeltaSeconds :type Float%20%28single-precision%29)))

(event EventInteract
  (params (Player_ref :type BP%20Third%20Person%20Character%20Object%20Reference))
  (if (Variables|Default|GetEnd_dialogue)
    (Widget|RemovefromParent (Variables|Default|GetDialogue_widget))
    (Variables|Default|SetEnd_dialogue false)
    (Variables|Default|SetDialogue_widget 0)
    (else
      (Utilities|IsValid (Variables|Default|GetDialogue_widget)
        (:Is%20Valid
          (bind _returnvalue (Utilities|GetDataTableRow (Variables|Default|GetData%20Table) (Variables|Default|GetRow%20Name))
            (:then
              (Default|UpdateDialogue (Variables|Default|GetDialogue_widget) (.Dialogue (Utilities|Struct|BreakDialogue_Structure _returnvalue)))
              (Variables|Default|SetRow%20Name (.Row (Utilities|Struct|BreakDialogue_Structure _returnvalue)))
              (Variables|Default|SetData%20Table (.Datatable (Utilities|Struct|BreakDialogue_Structure _returnvalue)))
              (Variables|Default|SetEnd_dialogue (.EndDialogue (Utilities|Struct|BreakDialogue_Structure _returnvalue))))))
        (:Is%20Not%20Valid
          (bind _returnvalue_2 (Utilities|GetDataTableRow (Variables|Default|GetData%20Table) (Variables|Default|GetRow%20Name))
            (:then
              (bind _returnvalue_3 (UserInterface|CreateWidget "/Game/DIalogue/WB_Dialogue.WB_Dialogue_C" 0 (Utilities|Text|ToText(Name) (Variables|Default|GetName)) (.Dialogue (Utilities|Struct|BreakDialogue_Structure _returnvalue_2))))
              (bind _output_get (Variables|Default|SetDialogue_widget _returnvalue_3))
              (UserInterface|Viewport|AddtoViewport _output_get 0)
              (Variables|Default|SetRow%20Name (.Row (Utilities|Struct|BreakDialogue_Structure _returnvalue_2)))
              (Variables|Default|SetData%20Table (.Datatable (Utilities|Struct|BreakDialogue_Structure _returnvalue_2)))
              (Variables|Default|SetEnd_dialogue (.EndDialogue (Utilities|Struct|BreakDialogue_Structure _returnvalue_2))))))))))