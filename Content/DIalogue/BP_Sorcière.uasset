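; Witch (Sorcière) dialogue Blueprint that prints lines for a quest and for ingredient-related responses.
; Five custom events cover the quest, first, second, third and non-ingredient cases, each incrementing an index into its own string array and showing that entry via PrintString.
; TalkQuest and TalkFirstIngredient both reset the first-ingredient index, so that dialogue repeats one line, which a comment marks as unfinished.
; No event checks array bounds.
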(event EventBeginPlay)

(event Collision|EventActorBeginOverlap
  (params (OtherActor :type Actor%20Object%20Reference)))

(event EventTick
  (params (DeltaSeconds :type Float%20%28single-precision%29)))

(event EventTalkQuest
  (Math|Integer|IncrementInt (Variables|Quest|GetTalk_Index)
    (:%20%20
      (Development|PrintString (Utilities|Array|Get(acopy) (Variables|Quest|GetDialogue_quest) (Variables|Quest|GetTalk_Index)))
      (Variables|First_Ingredient|SetTalk_First_Index -1))))

(event EventTalkFirstIngredient
  (Math|Integer|IncrementInt (Variables|First_Ingredient|GetTalk_First_Index)
    (:%20%20
      (Development|PrintString (Utilities|Array|Get(acopy) (Variables|First_Ingredient|GetDialogue_First) (Variables|First_Ingredient|GetTalk_First_Index)))
      ;[0.15 0.15 0.15 0.5] Réinitialise direct la première phrase, à régler demain
      (Variables|First_Ingredient|SetTalk_First_Index -1))))

(event EventTalkSecondIngredient
  (Math|Integer|IncrementInt (Variables|SecondIngredient|GetSecond_Index)
    (:%20%20
      (Development|PrintString (Utilities|Array|Get(acopy) (Variables|Second_Ingredient|GetDialogue_Second) (Variables|SecondIngredient|GetSecond_Index))))))

(event EventTalkThirdIngredient
  (Math|Integer|IncrementInt (Variables|ThirdIngredient|GetThird_Index)
    (:%20%20
      (Development|PrintString (Utilities|Array|Get(acopy) (Variables|Third_Ingredient|GetDialogue_Third) (Variables|ThirdIngredient|GetThird_Index))))))

(event EventTalkNonIngredient
  (Math|Integer|IncrementInt (Variables|Non|GetNon_Index)
    (:%20%20
      (Development|PrintString (Utilities|Array|Get(acopy) (Variables|Non|GetDialogue_Non) (Variables|Non|GetNon_Index))))))

(fn ConstructionScript)