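; BP_IngredientComponent is an ingredient inventory component that lets the player pick up BP_Ingredient actors.
; On BeginPlay it sizes the Ingredient array to one slot and adds a WB_Stack widget to display it.
; Pressing E runs a zero-length box trace at player 0's location to find a nearby ingredient.
; Its data fills any slot with zero Quantity, then the widget reloads and the actor is destroyed.
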(event EventBeginPlay
  (bind _returnvalue (UserInterface|CreateWidget "/Game/Interaction/Ingredient/Widget/WB_Stack.WB_Stack_C"))
  (Variables|Default|SetIngredientWidget _returnvalue)
  (Utilities|Array|Resize (Variables|Default|GetIngredient) 1)
  (Default|LoadIngredient (Variables|Default|GetIngredientWidget) self)
  (UserInterface|Viewport|AddtoViewport _returnvalue 0))

(event EventTick
  (params (DeltaSeconds :type Float%20%28single-precision%29)))

(event Input|KeyboardEvents|E
  (params (Key :type Key%20Structure))
  (bind _returnvalue (Game|GetPlayerCharacter 0))
  (bind _returnvalue_2 (Transformation|GetActorLocation _returnvalue))
  (bind _returnvalue_3 (- _returnvalue_2 ""))
  (:Pressed
    (bind _outhit (Collision|BoxTraceByChannel _returnvalue_3 _returnvalue_3 "100.000000,100.000000,100.000000" "0, 0, 0" "TraceTypeQuery1" false 0 "None"))
    (bind _asbp_ingredient (Utilities|Casting|CastToBP_Ingredient (.HitActor (Collision|BreakHitResult _outhit))))
    (for (_array_element _array_index) (Variables|Default|GetIngredient)
      (if (== (.Quantity (Utilities|Struct|BreakS_Ingredient_Structure _array_element)) 0)
        (Utilities|Array|SetArrayElem (Variables|Default|GetIngredient) _array_index (Variables|/Game/Interaction/Ingredient/Blueprint/BP_Ingredient.BP_Ingredient_C|GetIngredient _asbp_ingredient))
        (Default|LoadIngredient (Variables|Default|GetIngredientWidget) self)
        (Actor|DestroyActor _asbp_ingredient)))))