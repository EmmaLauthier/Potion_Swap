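; BP_Sorcière is the witch NPC, with three dialogues for ingredient hint, wrong ingredient and correct ingredient.
; Each Talk event, triggered from outside this graph, advances its own index through a dialogue array, showing speaker and line in a shared WB_Dialogue widget with a click sound.
; Past the last line it removes the widget and resets the index; the wrong-ingredient dialogue also clears the Test flag.
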(event EventBeginPlay)

(event Collision|EventActorBeginOverlap
  (params (OtherActor :type Actor%20Object%20Reference)))

(event EventTick
  (params (DeltaSeconds :type Float%20%28single-precision%29)))

(event EventTalkQuest
  ;[0.15 0.15 0.15 0.5 80] Indice Ingrédient Dialogue
  (Math|Integer|IncrementInt (Variables|Quest|GetTalk_Index)
    (:%20%20
      (if (< (Variables|Quest|GetTalk_Index) (Utilities|Array|Length (.Dialogue (Utilities|Struct|BreakS_DialogueStructure (Variables|Quest|GetDialogue_quest)))))
        (Variables|Default|GetUI
          (:then
            _)
          (:else
            (bind _returnvalue (UserInterface|CreateWidget "/Game/Interaction/DIalogue/WB_Dialogue.WB_Dialogue_C" (Game|GetPlayerController 0)))
            (bind _output_get (Variables|Default|SetUI _returnvalue))
            (UserInterface|Viewport|AddtoViewport _output_get 0)))
        (Rendering|Components|TextRender|SetText (Variables|/Game/Interaction/DIalogue/WB_Dialogue.WB_Dialogue_C|GetDialogueText (Variables|Default|GetUI)) (Utilities|Text|ToText(String) (Utilities|Array|Get(acopy) (.Dialogue (Utilities|Struct|BreakS_DialogueStructure (Variables|Quest|GetDialogue_quest))) (Variables|Quest|GetTalk_Index))))
        (Rendering|Components|TextRender|SetText (Variables|/Game/Interaction/DIalogue/WB_Dialogue.WB_Dialogue_C|GetName (Variables|Default|GetUI)) (Utilities|Text|ToText(Name) (.Name (Utilities|Struct|BreakS_DialogueStructure (Variables|Quest|GetDialogue_quest)))))
        (Audio|PlaySound2D "/Engine/VREditor/Sounds/UI/Click_on_Button.Click_on_Button" 1.0 1.0 0.0 0 0)
        (else
          (Variables|Default|GetUI
            (:then
              (Widget|RemovefromParent (Variables|Default|GetUI))
              (Variables|Quest|SetTalk_Index -1)
              (Variables|Default|SetUI 0))
            (:else)))))))

(event EventTalkNonIngredient
  ;[0.15 0.15 0.15 0.5 80] Mauvais Ingrédient Dialogue
  (Math|Integer|IncrementInt (Variables|Non|GetNon_Index)
    (:%20%20
      (if (< (Variables|Non|GetNon_Index) (Utilities|Array|Length (.Dialogue (Utilities|Struct|BreakS_DialogueStructure (Variables|Non|GetDialogue_Non)))))
        (Variables|Default|GetUI
          (:then
            _)
          (:else
            (bind _returnvalue (UserInterface|CreateWidget "/Game/Interaction/DIalogue/WB_Dialogue.WB_Dialogue_C" (Game|GetPlayerController 0)))
            (bind _output_get (Variables|Default|SetUI _returnvalue))
            (UserInterface|Viewport|AddtoViewport _output_get 0)))
        (Rendering|Components|TextRender|SetText (Variables|/Game/Interaction/DIalogue/WB_Dialogue.WB_Dialogue_C|GetDialogueText (Variables|Default|GetUI)) (Utilities|Text|ToText(String) (Utilities|Array|Get(acopy) (.Dialogue (Utilities|Struct|BreakS_DialogueStructure (Variables|Non|GetDialogue_Non))) (Variables|Non|GetNon_Index))))
        (Rendering|Components|TextRender|SetText (Variables|/Game/Interaction/DIalogue/WB_Dialogue.WB_Dialogue_C|GetName (Variables|Default|GetUI)) (Utilities|Text|ToText(Name) (.Name (Utilities|Struct|BreakS_DialogueStructure (Variables|Non|GetDialogue_Non)))))
        (Audio|PlaySound2D "/Engine/VREditor/Sounds/UI/Click_on_Button.Click_on_Button" 1.0 1.0 0.0 0 0)
        (else
          (Variables|Default|GetUI
            (:then
              (Widget|RemovefromParent (Variables|Default|GetUI))
              (Variables|Non|SetNon_Index -1)
              (Variables|Default|SetUI 0)
              (Variables|Default|SetTest false))
            (:else)))))))

(event EventTalkFirstIngredient
  ;[0.15 0.15 0.15 0.5 80] Bon Ingrédient Dialogue
  (Math|Integer|IncrementInt (Variables|First_Ingredient|GetTalk_First_Index)
    (:%20%20
      (if (< (Variables|First_Ingredient|GetTalk_First_Index) (Utilities|Array|Length (.Dialogue (Utilities|Struct|BreakS_DialogueStructure (Variables|First_Ingredient|GetDialogue_First)))))
        (Variables|Default|GetUI
          (:then
            _)
          (:else
            (bind _returnvalue (UserInterface|CreateWidget "/Game/Interaction/DIalogue/WB_Dialogue.WB_Dialogue_C" (Game|GetPlayerController 0)))
            (bind _output_get (Variables|Default|SetUI _returnvalue))
            (UserInterface|Viewport|AddtoViewport _output_get 0)))
        (Rendering|Components|TextRender|SetText (Variables|/Game/Interaction/DIalogue/WB_Dialogue.WB_Dialogue_C|GetDialogueText (Variables|Default|GetUI)) (Utilities|Text|ToText(String) (Utilities|Array|Get(acopy) (.Dialogue (Utilities|Struct|BreakS_DialogueStructure (Variables|First_Ingredient|GetDialogue_First))) (Variables|First_Ingredient|GetTalk_First_Index))))
        (Rendering|Components|TextRender|SetText (Variables|/Game/Interaction/DIalogue/WB_Dialogue.WB_Dialogue_C|GetName (Variables|Default|GetUI)) (Utilities|Text|ToText(Name) (.Name (Utilities|Struct|BreakS_DialogueStructure (Variables|First_Ingredient|GetDialogue_First)))))
        (Audio|PlaySound2D "/Engine/VREditor/Sounds/UI/Click_on_Button.Click_on_Button" 1.0 1.0 0.0 0 0)
        (else
          (Variables|Default|GetUI
            (:then
              (Widget|RemovefromParent (Variables|Default|GetUI))
              (Variables|First_Ingredient|SetTalk_First_Index -1)
              (Variables|Default|SetUI 0))
            (:else)))))))

(fn ConstructionScript)