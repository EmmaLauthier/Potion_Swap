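; BP_Rob is the player character, with Enhanced Input movement, jumping and a pause menu, plus an Aim function left empty.
; Pressing F checks its ingredient component's entries against overlapping BP_Sorcière witches to choose quest, missing-ingredient or success dialogue.
; Success reveals Potion-tagged ingredients and sets Endgame.
; A potion entry can then open Story_map with the Endgame option.
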(event Input|EnhancedActionEvents|EnhancedInputActionIA_Pause
  (params (ActionValue :type Boolean) (ElapsedSeconds :type Float%20%28double-precision%29) (TriggeredSeconds :type Float%20%28double-precision%29) (InputAction :type Input%20Action%20Object%20Reference :default "/Game/Input/Actions/IA_Pause.IA_Pause"))
  (bind _returnvalue (Game|GetPlayerController 0))
  ;[0.15 0.15 0.15 0.5 100] Pause Menu
  (bind _returnvalue_2 (UserInterface|CreateWidget "/Game/UI/WB_PauseMenu.WB_PauseMenu_C"))
  (UserInterface|Viewport|AddtoViewport _returnvalue_2 0)
  (Variables|/Script/Engine.PlayerController|SetbShowMouseCursor _returnvalue true)
  (Input|SetInputModeUIOnly _returnvalue 0 "DoNotLock" false)
  (Game|SetGamePaused true))

(event Input|EnhancedActionEvents|EnhancedInputActionINP_Move
  (params (ActionValue :type Vector%202D%20Structure) (ElapsedSeconds :type Float%20%28double-precision%29) (TriggeredSeconds :type Float%20%28double-precision%29) (InputAction :type Input%20Action%20Object%20Reference :default "/Game/Characters/Rob/Input/INP_Move.INP_Move"))
  (bind _returnvalue (Pawn|GetControlRotation :!class /Script/Engine.Pawn))
  (:Triggered
    (Pawn|Input|AddMovementInput (Math|Vector|GetRightVector (Pawn|GetControlRotation :!class /Script/Engine.Pawn)) (.x ActionValue) false)
    (Pawn|Input|AddMovementInput (Math|Vector|GetForwardVector (Math|Rotator|MakeRotator (.roll _returnvalue) 0.0 (.yaw _returnvalue))) (.y ActionValue) false)))

(event Input|EnhancedActionEvents|EnhancedInputActionINP_Jump
  (params (ActionValue :type Boolean) (ElapsedSeconds :type Float%20%28double-precision%29) (TriggeredSeconds :type Float%20%28double-precision%29) (InputAction :type Input%20Action%20Object%20Reference :default "/Game/Characters/Rob/Input/INP_Jump.INP_Jump"))
  (:Started
    (Character|Jump))
  (:Completed
    (Character|StopJumping)))

(event Input|EnhancedActionEvents|EnhancedInputActionIA_MouseLook
  (params (ActionValue :type Vector%202D%20Structure) (ElapsedSeconds :type Float%20%28double-precision%29) (TriggeredSeconds :type Float%20%28double-precision%29) (InputAction :type Input%20Action%20Object%20Reference :default "/Game/Input/Actions/IA_MouseLook.IA_MouseLook"))
  (CallFunction|Aim (.x ActionValue) (.y ActionValue)))

(event EventBeginPlay
  (bind _returnvalue (Game|GetPlayerController 0))
  (bind _returnvalue_2 (PlayerController|LocalPlayerSubsystems|GetEnhancedInputLocalPlayerSubsystem _returnvalue))
  (Utilities|IsValid _returnvalue_2
    (:Is%20Valid
      (Input|AddMappingContext _returnvalue_2 "/Game/Characters/Rob/Input/IMC_ThirdPerson.IMC_ThirdPerson" 0 "(bIgnoreAllPressedKeysUntilRelease=True,bForceImmediately=False,bNotifyUserSettings=False)"))))

(event Collision|EventActorBeginOverlap
  (params (OtherActor :type Actor%20Object%20Reference)))

(event EventTick
  (params (DeltaSeconds :type Float%20%28single-precision%29)))

(event Input|KeyboardEvents|F
  (params (Key :type Key%20Structure :default "None"))
  ;[0.15 0.15 0.15 0.5 100] Dialogue System
  (:Pressed
    (for _array_element (Variables|/Game/Interaction/Ingredient/Blueprint/BP_IngredientComponent.BP_IngredientComponent_C|GetIngredient (Variables|Default|GetBP_IngredientComponent))
      (for _array_element_2 (Collision|GetOverlappingActors "/Game/Interaction/DIalogue/BP_Sorcière.BP_Sorcière_C" :!class /Script/Engine.Actor)
        (if (.IsOk (Utilities|Struct|BreakS_Ingredient_Structure _array_element))
          (Class|BPIDialogue|TalkFirstIngredient(Message) _array_element_2)
          (bind _outactors (Actor|GetAllActorsOfClasswithTag "/Game/Interaction/Ingredient/Blueprint/BP_Ingredient.BP_Ingredient_C" "Potion"))
          (Rendering|SetActorHiddenInGame _outactors false)
          (Variables|Default|SetEndgame true)
          (elif (and (== (Variables|Default|GetEndgame) false) (== (.Quantity (Utilities|Struct|BreakS_Ingredient_Structure _array_element)) 0))
            (Class|BPIDialogue|TalkQuest(Message) _array_element_2)
            (elif (.IsPotion (Utilities|Struct|BreakS_Ingredient_Structure _array_element))
              (Game|OpenLevel(byName) "Story_map" true "Endgame")
              (elif (== (.IsOk (Utilities|Struct|BreakS_Ingredient_Structure _array_element)) false)
                (Class|BPIDialogue|TalkNonIngredient(Message) _array_element_2)))))))))

(fn ConstructionScript)

(fn Aim
  (params (X%20Axis :type Float%20%28single-precision%29) (Y%20Axis :type Float%20%28double-precision%29)))